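; Flickering light actor that blinks its PointLight on and off in a continuous, regular pattern.
; BeginPlay starts a custom event that toggles the light's visibility, then re-triggers itself after a Delay, forming a timer loop without Tick.
; The delay depends on the new state, so the light stays visible longer than it stays dark.
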(event `self.ReceiveBeginPlay`
  (`self.EventToggleLight`))

(event `EventToggleLight`
  (`SceneComponent.ToggleVisibility` (`self.PointLight`) false)
  (if (`SceneComponent.IsVisible` (`self.PointLight`))
    (bind _output_get (set `self.TimerTime` 1.0))
    (`KismetSystemLibrary.Delay` _output_get)
    (`self.EventToggleLight`)
    (else
      (bind _output_get_2 (set `self.TimerTime` 0.5))
      (`KismetSystemLibrary.Delay` _output_get_2)
      (`self.EventToggleLight`))))

(fn `UserConstructionScript`)